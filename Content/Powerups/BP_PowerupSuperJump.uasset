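; Super Jump powerup that temporarily doubles the jump height velocity of the actor it activates on.
; On activation it stores that actor and multiplies its CharacterMovementComponent JumpZVelocity by two.
; On expiry it halves the velocity again if the actor is still valid, then runs the parent powerup's expiry logic.
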(event EventOnActivated
  (params (ActiveFor :type Actor%20Object%20Reference))
  (bind _output_get (Variables|Default|SetActiveFor ActiveFor))
  (Variables|/Script/Engine.CharacterMovementComponent|SetJumpZVelocity (Actor|GetComponentbyClass _output_get "/Script/Engine.CharacterMovementComponent") (* (Variables|/Script/Engine.CharacterMovementComponent|GetJumpZVelocity (Actor|GetComponentbyClass _output_get "/Script/Engine.CharacterMovementComponent")) 2.0)))

(event EventOnExpired
  (bind _activefor (Variables|Default|GetActiveFor))
  (bind _returnvalue (Actor|GetComponentbyClass _activefor "/Script/Engine.CharacterMovementComponent"))
  (Utilities|IsValid (Variables|Default|GetActiveFor)
    (:Is%20Valid
      (Variables|/Script/Engine.CharacterMovementComponent|SetJumpZVelocity _returnvalue (/ (Variables|/Script/Engine.CharacterMovementComponent|GetJumpZVelocity _returnvalue) 2.0)))
    (:Is%20Not%20Valid
      _))
  (|CallParentFunction))

(fn ConstructionScript
  (|CallParentFunction))