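; Super speed powerup that doubles the walk speed of the actor it activates on until it expires.
; OnActivated stores that actor and sets its CharacterMovementComponent's MaxWalkSpeed to twice GetMaxSpeed.
; OnExpired sets MaxWalkSpeed to half the then-current GetMaxSpeed rather than restoring a saved value, then calls the parent's expiry logic.
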(event EventOnActivated
  (params (ActiveFor :type Actor%20Object%20Reference))
  (bind _output_get (Variables|Default|SetActiveFor ActiveFor))
  (Utilities|IsValid (Actor|GetComponentbyClass _output_get "/Script/Engine.CharacterMovementComponent")
    (:Is%20Valid
      (Variables|/Script/Engine.CharacterMovementComponent|SetMaxWalkSpeed (Actor|GetComponentbyClass _output_get "/Script/Engine.CharacterMovementComponent") (* (Class|MovementComponent|GetMaxSpeed (Actor|GetComponentbyClass _output_get "/Script/Engine.CharacterMovementComponent")) 2.0)))))

(event EventOnExpired
  (bind _activefor (Variables|Default|GetActiveFor))
  (bind _returnvalue (Actor|GetComponentbyClass _activefor "/Script/Engine.CharacterMovementComponent"))
  (Utilities|IsValid (Variables|Default|GetActiveFor)
    (:Is%20Valid
      (Utilities|IsValid _returnvalue
        (:Is%20Valid
          (Variables|/Script/Engine.CharacterMovementComponent|SetMaxWalkSpeed _returnvalue (/ (Class|MovementComponent|GetMaxSpeed _returnvalue) 2.0)))
        (:Is%20Not%20Valid
          _)))
    (:Is%20Not%20Valid
      _))
  (|CallParentFunction))

(fn ConstructionScript)